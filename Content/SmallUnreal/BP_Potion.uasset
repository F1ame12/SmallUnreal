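; BP_Potion is a potion actor that heals the player in exchange for credits.
; Its Intraction function casts the other actor to SCharacter and rejects it if that fails or health is already full.
; If the character's credit component covers CreditCost, it changes the credits by that cost and applies HealVal through the attribute component, returning the result.
; The event graph and construction script are empty.
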(event EventBeginPlay)

(event Collision|EventActorBeginOverlap
  (params (OtherActor :type Actor%20Object%20Reference)))

(event EventTick
  (params (DeltaSeconds :type Float%20%28single-precision%29)))

(fn ConstructionScript)

(fn Intraction
  (params (OverlappedComponent :type Primitive%20Component%20Object%20Reference) (OtherActor :type Actor%20Object%20Reference) (OtherComp :type Primitive%20Component%20Object%20Reference) (OtherBodyIndex :type Integer) (bFromSweep :type Boolean) (SweepResult :type Hit%20Result%20Structure%20%28by%20ref%29))
  (bind _creditcost (Variables|Default|GetCreditCost))
  ;[1 1 1] 仅玩家可触发
  (bind _asscharacter (Utilities|Casting|CastToSCharacter OtherActor)
    (:then
      (bind _returnvalue (Class|SAttributeComponent|GetAttributeComponent _asscharacter))
      ;[1 1 1] 满血时无法触发
      (bind _returnvalue_2 (Class|SAttributeComponent|GetMaxHealth _returnvalue))
      (if (Math|Float|NearlyEqual(Float) _returnvalue_2 (Variables|/Script/SmallUnreal.SAttributeComponent|GetHealth _returnvalue) 1e-06)
        (return false)
        (else
          ;[1 1 1] 需要有足够的积分
          (if (>= (Class|CreditComponent|GetCredits (Variables|/Script/SmallUnreal.SCharacter|GetCreditComp _asscharacter)) _creditcost)
            (bind _result (Math|Float|NegateFloat _creditcost)
              (:%20%20
                (Class|CreditComponent|ChangeCreditAmount (Variables|/Script/SmallUnreal.SCharacter|GetCreditComp _asscharacter) _result)
                (bind _returnvalue_3 (Class|SAttributeComponent|ApplyHealthChange _returnvalue self (Variables|Default|GetHealVal)))
                (return _returnvalue_3)))))))
    (:CastFailed
      (return false))))