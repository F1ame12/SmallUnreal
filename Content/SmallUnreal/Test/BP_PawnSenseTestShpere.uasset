(event OnSeePawn(PawnSensing)
  (params (Pawn :type Pawn%20Object%20Reference))
  (Utilities|FlowControl|DoOnce false :!label _label
    (:Completed
      (Development|PrintString "shpere see you!" true true "(R=0.904426,G=0.030131,B=1.000000,A=1.000000)" 4.0)
      (bind _aswbp_actor_talk_widget (Utilities|Casting|CastToWBP_ActorTalkWidget (UserInterface|GetWidget (Variables|Default|GetWidget))))
      (Rendering|Components|TextRender|SetText (Variables|/Game/SmallUnreal/UI/WBP_ActorTalkWidget.WBP_ActorTalkWidget_C|GetTextBlock _aswbp_actor_talk_widget) "我看到你了！")
      (Rendering|SetVisibility (Variables|Default|GetWidget) true false)
      (Utilities|FlowControl|Delay 3.0)
      (Rendering|SetVisibility (Variables|Default|GetWidget) false false)
      (Utilities|FlowControl|Delay 3.0)
      (goto _label Reset))))

(event OnHearNoise(PawnSensing)
  (params (Instigator :type Pawn%20Object%20Reference) (Location :type Vector%20%28by%20ref%29 :default "0, 0, 0") (Volume :type Float%20%28single-precision%29))
  (Development|PrintString "shpere hear you!" true true "(R=0.904426,G=0.030131,B=1.000000,A=1.000000)" 4.0))

(event EventBeginPlay)

(event Collision|EventActorBeginOverlap
  (params (OtherActor :type Actor%20Object%20Reference)))

(event EventTick
  (params (DeltaSeconds :type Float%20%28single-precision%29)))

(fn ConstructionScript)