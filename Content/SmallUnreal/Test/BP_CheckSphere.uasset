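; BP_CheckSphere is a test actor that periodically detects nearby objects and reports them on screen.
; On BeginPlay it plays the CheckActor timeline, whose Finished output runs a multi sphere trace for WorldDynamic and Pawn objects at the actor's location with debug drawing.
; It prints the name of each hit actor, then restarts the timeline, using it as a repeating timer.
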(event EventBeginPlay
  (bind _self self)
  (bind _returnvalue (Transformation|GetActorLocation _self))
  (Timeline|CheckActor Play
    (:Finished
      (bind _outhits (Collision|MultiSphereTraceForObjects _returnvalue _returnvalue 2.5e+02 (Utilities|Array|MakeArray "ObjectTypeQuery2" "ObjectTypeQuery3") false 0 "ForDuration"))
      (for _array_element _outhits
        (Development|PrintString (Utilities|String|Append (Utilities|String|ToString(Text) (Utilities|Text|MakeLiteralText "check obj----")) (Utilities|GetObjectName (.HitActor (Collision|BreakHitResult _array_element)))) true true "(R=1.000000,G=0.328682,B=0.208813,A=1.000000)"))
      (Timeline|CheckActor PlayFromStart))))

(event Collision|EventActorBeginOverlap
  (params (OtherActor :type Actor%20Object%20Reference)))

(event EventTick
  (params (DeltaSeconds :type Float%20%28single-precision%29)))

(fn ConstructionScript)