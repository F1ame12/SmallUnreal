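; BP_MinionRange is an AI minion Blueprint, presumably the ranged type, that manages its overhead health bar widget.
; It creates the bar attached to itself on BeginPlay and removes it on Destroyed.
; Each Tick, a visibility trace between its eyes and the player's shows the bar only when unobstructed.
; Overlap with another instigator's magic projectile collapses the bar, though the next Tick re-evaluates visibility.
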(event EventBeginPlay
  (bind _returnvalue (UserInterface|CreateWidget "/Game/SmallUnreal/UI/BP_ActorTopHealthBar_Widget.BP_ActorTopHealthBar_Widget_C" 0 self (Math|Float|MakeLiteralFloat 7e+01)))
  (Variables|Default|SetTopHealthBar _returnvalue)
  (Widget|SetVisibility (Variables|Default|GetTopHealthBar) "HitTestInvisible")
  (UserInterface|Viewport|AddtoViewport (Variables|Default|GetTopHealthBar) 0))

(event Collision|EventActorBeginOverlap
  (params (OtherActor :type Actor%20Object%20Reference))
  (bind _asabase_magic_projectile (Utilities|Casting|CastToABaseMagicProjectile OtherActor))
  (if (!= (Variables|/Script/Engine.Actor|GetInstigator _asabase_magic_projectile) self)
    (Widget|SetVisibility (Variables|Default|GetTopHealthBar) "Collapsed")))

(event EventTick
  (params (DeltaSeconds :type Float%20%28single-precision%29))
  (CallFunction|UpdateTopHealthBarVisiiblity))

(event EventDestroyed
  (Widget|RemovefromParent (Variables|Default|GetTopHealthBar)))

(fn ConstructionScript)

(fn UpdateTopHealthBarVisiiblity
  (bind _returnvalue (Game|Player|GetPlayerPawn 0))
  (bind _tophealthbar (Variables|Default|GetTopHealthBar))
  ;[1 1 1] 根据AI模型的视角位置与玩家模型的视角位置判断是否可见
  (bind _returnvalue_2 (Collision|LineTraceByChannel (.OutLocation (Actor|GetActorEyesViewPoint self)) (.OutLocation (Actor|GetActorEyesViewPoint _returnvalue)) "TraceTypeQuery1" false (Utilities|Array|MakeArray _returnvalue) "None"))
  (if _returnvalue_2
    (Widget|SetVisibility _tophealthbar "Collapsed")
    (else
      (Widget|SetVisibility _tophealthbar "HitTestInvisible"))))