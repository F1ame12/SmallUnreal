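; BP_HealPosion is a healing potion pickup that restores a fixed amount of health to the pawn that interacts with it.
; Interact checks the CanInteract flag and calls ApplyHealthChange on the instigator's SAttributeComponent.
; Only a successful heal hides the mesh, blocks further interaction and plays the HealCoolDown timeline.
; When the timeline finishes, the potion reappears, becomes interactable again and resets the timeline's time for reuse.
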(event EventBeginPlay
  (Variables|Default|SetbCanInteract true))

(event Collision|EventActorBeginOverlap
  (params (OtherActor :type Actor%20Object%20Reference)))

(event EventTick
  (params (DeltaSeconds :type Float%20%28single-precision%29)))

(event EventInteract
  (params (InstigatorPawn :type Pawn%20Object%20Reference))
  (bind _returnvalue (Actor|GetComponentbyClass InstigatorPawn "/Script/SmallUnreal.SAttributeComponent"))
  (if (Variables|Default|GetbCanInteract)
    (Utilities|IsValid _returnvalue
      (:Is%20Valid
        (bind _returnvalue_2 (Class|SAttributeComponent|ApplyHealthChange _returnvalue 2e+01))
        (if _returnvalue_2
          (Variables|Default|SetbCanInteract false)
          (Rendering|SetVisibility (Variables|Default|GetPosionMesh) false false)
          ;[1 1 1] 一定时间后重新显示物体并允许交互
          (Timeline|HealCoolDown Play
            (:Finished
              (Variables|Default|SetbCanInteract true)
              (Rendering|SetVisibility (Variables|Default|GetPosionMesh) true false)
              (Timeline|HealCoolDown SetNewTime))))))))

(fn ConstructionScript)